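; BP_BlackJack3DActor_Actor is a world actor that lets the player open a blackjack widget by walking up and interacting.
; Trigger box overlap with the player character toggles the interaction prompt widget, the IsInBox flag and input on the actor.
; Pressing E inside the box calls OnInteract, which creates the widget class named in the DataAsset, passes that asset to it and adds it to the viewport.
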(event `self.TriggerBox.OnComponentBeginOverlap`
  (params (OverlappedComponent :type "PrimitiveComponent Object Reference") (OtherActor :type "Actor Object Reference") (OtherComp :type "PrimitiveComponent Object Reference") (OtherBodyIndex :type Integer) (bFromSweep :type Boolean) (SweepResult :type "HitResult Structure (by ref)"))
  (if (== OtherActor (`GameplayStatics.GetPlayerCharacter` 0))
    (set `self.IsInBox` true)
    (`SceneComponent.SetVisibility` (`self.InteractionWidget`) true false)
    (`self.EnableInput` (`GameplayStatics.GetPlayerController` 0))))

(event `self.TriggerBox.OnComponentEndOverlap`
  (params (OverlappedComponent :type "PrimitiveComponent Object Reference") (OtherActor :type "Actor Object Reference") (OtherComp :type "PrimitiveComponent Object Reference") (OtherBodyIndex :type Integer))
  (if (== OtherActor (`GameplayStatics.GetPlayerCharacter` 0))
    (set `self.IsInBox` false)
    (`SceneComponent.SetVisibility` (`self.InteractionWidget`) false false)
    (`self.DisableInput` (`GameplayStatics.GetPlayerController` 0) null)))

(event `Key|E`
  (params (Key :type "Key Structure"))
  (:`Pressed`
    (`self.OnInteract`)))

(fn `OnInteract`
  (bind _dataasset (`self.DataAsset`))
  (if (`self.IsInBox`)
    (bind _returnvalue (`|CreateWidget` (`/Game/BlackJackBlueprint/Blueprints/Utils/BP_BlackJackVersion_DataAsset.WidgetClass` _dataasset) null _dataasset null))
    (`UserWidget.AddToViewport` _returnvalue 0)))

(fn `UserConstructionScript`)