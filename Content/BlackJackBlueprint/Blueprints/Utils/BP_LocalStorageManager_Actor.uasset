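; Actor that manages local save data for the blackjack game, storing the player's username and balance.
; On BeginPlay it checks the save slot and, if none exists, creates a custom SaveGame with a starting balance and writes it.
; Getter and setter functions reload the slot on every call, cast to the custom SaveGame, and setters write it straight back.
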(event `self.ReceiveBeginPlay`
  (`self.CheckForExistingSaveGame`))

(fn `CheckForExistingSaveGame`
  (bind _returnvalue (`GameplayStatics.DoesSaveGameExist` (`self.SlotName`)))
  (if (not _returnvalue)
    (bind _returnvalue_2 (`GameplayStatics.CreateSaveGameObject` "/Game/BlackJackBlueprint/Blueprints/Utils/BP_CustomSaveGame_SaveGameBlueprint.BP_CustomSaveGame_SaveGameBlueprint_C"))
    (set `/Game/BlackJackBlueprint/Blueprints/Utils/BP_CustomSaveGame_SaveGameBlueprint.Balance` 2000 _returnvalue_2)
    (`GameplayStatics.SaveGameToSlot` _returnvalue_2 (`self.SlotName`))))

(fn `GetBalance`
  (returns (Balance :type Integer))
  (bind _returnvalue (`GameplayStatics.LoadGameFromSlot` (`self.SlotName`)))
  (bind _asbp_custom_save_game_save_game_blueprint (cast `/Game/BlackJackBlueprint/Blueprints/Utils/BP_CustomSaveGame_SaveGameBlueprint` _returnvalue))
  (return (`/Game/BlackJackBlueprint/Blueprints/Utils/BP_CustomSaveGame_SaveGameBlueprint.Balance` _asbp_custom_save_game_save_game_blueprint)))

(fn `GetUsername`
  (returns (Username :type String))
  (bind _returnvalue (`GameplayStatics.LoadGameFromSlot` (`self.SlotName`)))
  (bind _asbp_custom_save_game_save_game_blueprint (cast `/Game/BlackJackBlueprint/Blueprints/Utils/BP_CustomSaveGame_SaveGameBlueprint` _returnvalue))
  (return (`/Game/BlackJackBlueprint/Blueprints/Utils/BP_CustomSaveGame_SaveGameBlueprint.Username` _asbp_custom_save_game_save_game_blueprint)))

(fn `SaveBalance`
  (params (Balance :type Integer))
  (bind _returnvalue (`GameplayStatics.LoadGameFromSlot` (`self.SlotName`)))
  (bind _asbp_custom_save_game_save_game_blueprint (cast `/Game/BlackJackBlueprint/Blueprints/Utils/BP_CustomSaveGame_SaveGameBlueprint` _returnvalue))
  (set `/Game/BlackJackBlueprint/Blueprints/Utils/BP_CustomSaveGame_SaveGameBlueprint.Balance` Balance _asbp_custom_save_game_save_game_blueprint)
  (`GameplayStatics.SaveGameToSlot` _asbp_custom_save_game_save_game_blueprint (`self.SlotName`)))

(fn `SaveUsername`
  (params (Username :type String))
  (bind _returnvalue (`GameplayStatics.LoadGameFromSlot` (`self.SlotName`)))
  (bind _asbp_custom_save_game_save_game_blueprint (cast `/Game/BlackJackBlueprint/Blueprints/Utils/BP_CustomSaveGame_SaveGameBlueprint` _returnvalue))
  (set `/Game/BlackJackBlueprint/Blueprints/Utils/BP_CustomSaveGame_SaveGameBlueprint.Username` Username _asbp_custom_save_game_save_game_blueprint)
  (`GameplayStatics.SaveGameToSlot` _asbp_custom_save_game_save_game_blueprint (`self.SlotName`)))

(fn `UserConstructionScript`)