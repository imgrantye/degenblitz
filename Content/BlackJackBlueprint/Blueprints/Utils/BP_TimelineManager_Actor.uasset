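; Actor that runs timelines for card animations in the blackjack game on behalf of the main game widget, which is passed in at initialization.
; Each event plays a timeline from the start for one animation, such as dealing, shifting hands, flipping the dealer's card or clearing the table.
; Every update feeds track progress to the widget's matching update event, and dealing and clearing also notify it when finished.
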(event `InitializeWidgetInstance`
  (params (MainGameWidgetReference :type "/Game/BlackJackBlueprint/Blueprints/WBP_MainGame_UserWidget Object Reference"))
  (set `self.MainGameWidgetInstance` MainGameWidgetReference))

(event `MoveShuffledCardsTimelineEvent`
  (bind (_direction _newtrack_0) (`Timeline|MoveShuffledCardsTimeline` :!via `PlayFromStart`)
    (:`Update`
      (`/Game/BlackJackBlueprint/Blueprints/WBP_MainGame_UserWidget.MoveSpawnedCardUpdateEvent` (`self.MainGameWidgetInstance`) _newtrack_0))))

(event `MoveCardFromDeckToHandEvent`
  (params (panelReference :type "PanelSlot Object Reference") (destination :type "Vector2D Structure") (source :type "Vector2D Structure") (cardName :type String) (faceUp :type Boolean))
  (bind _maingamewidgetinstance (`self.MainGameWidgetInstance`))
  (bind (_direction _newtrack_0) (`Timeline|MoveCardFromDeckToHandTimeline` :!via `PlayFromStart`)
    (:`Update`
      (`/Game/BlackJackBlueprint/Blueprints/WBP_MainGame_UserWidget.MoveCardFromDeckToHandUpdateEvent` _maingamewidgetinstance _newtrack_0 panelReference source destination cardName faceUp))
    (:`Finished`
      (`/Game/BlackJackBlueprint/Blueprints/WBP_MainGame_UserWidget.MovingCardToDealerHandFinishedEvent` _maingamewidgetinstance))))

(event `MoveCardsInPlayerDeckEvent`
  (bind (_direction _newtrack_0) (`Timeline|MoveCardsInPlayerDeckTimeline` :!via `PlayFromStart`)
    (:`Update`
      (`/Game/BlackJackBlueprint/Blueprints/WBP_MainGame_UserWidget.MoveCardsAlreadyInPlayerDeckUpdateEvent` (`self.MainGameWidgetInstance`) _newtrack_0))))

(event `FlipDealerFirstCardEvent`
  (bind (_direction _newtrack_0) (`Timeline|FlipDealerFirstCardTimeline` :!via `PlayFromStart`)
    (:`Update`
      (`/Game/BlackJackBlueprint/Blueprints/WBP_MainGame_UserWidget.FlipDealerFirstCardUpdateEvent` (`self.MainGameWidgetInstance`) _newtrack_0))))

(event `MoveCardsInDealerDeckEvent`
  (bind (_direction _newtrack_0) (`Timeline|MoveCardsInDealerDeckTimeline` :!via `PlayFromStart`)
    (:`Update`
      (`/Game/BlackJackBlueprint/Blueprints/WBP_MainGame_UserWidget.MoveCardsAlreadyInDealerHandUpdateEvent` (`self.MainGameWidgetInstance`) _newtrack_0))))

(event `MoveCardsOutsideEvent`
  (bind _maingamewidgetinstance (`self.MainGameWidgetInstance`))
  (bind (_direction _newtrack_0) (`Timeline|MoveCardsOutsideTimeline` :!via `PlayFromStart`)
    (:`Update`
      (`/Game/BlackJackBlueprint/Blueprints/WBP_MainGame_UserWidget.MoveCardsOutsideUpdateEvent` _maingamewidgetinstance _newtrack_0))
    (:`Finished`
      (`/Game/BlackJackBlueprint/Blueprints/WBP_MainGame_UserWidget.MovingCardsOutsideFinishedEvent` _maingamewidgetinstance))))

(event `MoveCardFromHandToHandEvent`
  (params (source :type "Vector2D Structure") (destination :type "Vector2D Structure") (cardName :type String))
  (bind (_direction _newtrack_0) (`Timeline|MoveCardFromHandToHandTimeline` :!via `PlayFromStart`)
    (:`Update`
      (`/Game/BlackJackBlueprint/Blueprints/WBP_MainGame_UserWidget.MoveCardFromHandToHandUpdateEvent` (`self.MainGameWidgetInstance`) source destination cardName _newtrack_0))))

(event `MoveCardsAlreadyInNPCHandEvent`
  (params (NPCIndex :type Integer))
  (bind (_direction _newtrack_0) (`Timeline|MoveCardsAlreadyInNPCHandTimeline` :!via `PlayFromStart`)
    (:`Update`
      (`/Game/BlackJackBlueprint/Blueprints/WBP_MainGame_UserWidget.MoveCardsAlreadyInNPCDeckUpdateEvent` (`self.MainGameWidgetInstance`) _newtrack_0 NPCIndex))))

(fn `UserConstructionScript`)